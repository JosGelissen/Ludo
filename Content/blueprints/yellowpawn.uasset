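; Clickable pawn for a turn-based dice board game that moves around a looping spline track.
; On click it checks GS_Mejn's turn and permissions, then enters the board or moves by the BP_Dice throw.
; Movement steps one spline point per delayed recursive call, wrapping at the track's end.
; It updates board positions in the game state and reports placement, landing hits, house arrival and finished moves to GM_Mejn.
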(event `self.ReceiveBeginPlay`)

(event `pawnmoves`
  (params (moves :type Integer))
  (if (> moves 0)
    (`KismetSystemLibrary.Delay` 0.3)
    (`self.Move Pawn` moves)
    (else
      (bind _asgm_mejn (cast `/Game/blueprints/GM_Mejn` (`GameplayStatics.GetGameMode`)))
      (`/Game/blueprints/GM_Mejn.pawnmoved` _asgm_mejn))))

(event `self.ReceiveActorOnClicked`
  (params (ButtonPressed :type "Key Structure"))
  (bind _asgs_mejn (cast `/Game/blueprints/GS_Mejn` (`GameplayStatics.GetGameState`)))
  (bind _turnactions (`/Game/blueprints/GS_Mejn.turnactions` _asgs_mejn))
  (switch `string` (`BlueprintMapLibrary.Map_Find` _turnactions "turn")
    (:`yellow`
      (set `self.stats` (`/Game/blueprints/GS_Mejn.yellowstats` _asgs_mejn)))
    (:`green`
      (set `self.stats` (`/Game/blueprints/GS_Mejn.greenstats` _asgs_mejn)))
    (:`blue`
      (set `self.stats` (`/Game/blueprints/GS_Mejn.bluestats` _asgs_mejn)))
    (:`red`
      (set `self.stats` (`/Game/blueprints/GS_Mejn.redstats` _asgs_mejn))))
  ;[1 1 1] check if it is my colors turn
  (if (`KismetStringLibrary.EqualEqual_StrStr` (`BlueprintMapLibrary.Map_Find` _turnactions "turn") (`self.mycolor`))
    ;[1 1 1] check if i'm allowed to be moved
    (if (`KismetStringLibrary.EqualEqual_StrStr` (`BlueprintMapLibrary.Map_Find` _turnactions "movepawn") "true")
      (bind _outactors (`GameplayStatics.GetAllActorsOfClass` "/Game/blueprints/BP_Dice.BP_Dice_C"))
      (`self.pawnmoves` (`/Game/blueprints/BP_Dice.dicethrow` (`|GetArrayItem` _outactors)))
      (else
        ;[1 1 1] check if i'm allowed to go on the board
        (if (`KismetStringLibrary.EqualEqual_StrStr` (`BlueprintMapLibrary.Map_Find` _turnactions "goonboard") "true")
          (`self.PawnonBoard`))))
    (else
      (`KismetSystemLibrary.PrintString` "it is not your turn"))))

(fn `Move Pawn`
  (params (moves :type Integer))
  (bind _returnvalue (- moves 1))
  (bind _stats (`self.stats`))
  (bind _returnvalue_2 (+ (`self.currentsplinepoint`) 1))
  ;[1 1 1] move pawn by one and update currentspline point and moves left
  (`self.K2_SetActorLocation` (`SplineComponent.GetLocationAtSplinePoint` (`/Game/blueprints/BP_Splinetrack.Spline` (`self.track`)) _returnvalue_2 "World"))
  (if (== (- _returnvalue_2 (`BlueprintMapLibrary.Map_Find` _stats "correction")) (`BlueprintMapLibrary.Map_Find` _stats "end"))
    (`KismetSystemLibrary.PrintString` "inhuis")
    (bind _asgm_mejn (cast `/Game/blueprints/GM_Mejn` (`GameplayStatics.GetGameMode`)))
    (`/Game/blueprints/GM_Mejn.pawninhouse` _asgm_mejn self)
    (else
      ;;[1 1 1] check if the end of track is reached
      (if (== _returnvalue_2 40)
        (set `self.currentsplinepoint` 0))
      (bind _output_get (set `self.currentsplinepoint` _returnvalue_2))
      ;[1 1 1] updategamestatewith new position amnd check if there already is a pawn
      (bind _asgs_mejn (cast `/Game/blueprints/GS_Mejn` (`GameplayStatics.GetGameState`)))
      (bind _pawnsonboard (`/Game/blueprints/GS_Mejn.pawnsonboard` _asgs_mejn))
      (`BlueprintMapLibrary.Map_Remove` _pawnsonboard self)
      ;[1 1 1] check if i hit a pawn and tell the game mode
      (if (== _returnvalue 0)
        (bind _values (`BlueprintMapLibrary.Map_Values` _pawnsonboard))
        (for (_array_element _array_index) _values
          (if (== _array_element _output_get)
            (bind _keys (`BlueprintMapLibrary.Map_Keys` _pawnsonboard))
            (bind _asgm_mejn_2 (cast `/Game/blueprints/GM_Mejn` (`GameplayStatics.GetGameMode`)))
            (`/Game/blueprints/GM_Mejn.pawnhit` _asgm_mejn_2 (`|GetArrayItem` _keys _array_index)))))
      (`BlueprintMapLibrary.Map_Add` _pawnsonboard self _output_get)
      (`self.pawnmoves` _returnvalue))))

(fn `PawnonBoard`
  (bind _value (`BlueprintMapLibrary.Map_Find` (`self.stats`) "start"))
  (`KismetSystemLibrary.PrintString` "pawn on board")
  ;[1 1 1] placement of pawn on board
  (`self.K2_SetActorLocation` (`SplineComponent.GetLocationAtSplinePoint` (`/Game/blueprints/BP_Splinetrack.Spline` (`self.track`)) _value "World"))
  (bind _output_get (set `self.currentsplinepoint` _value))
  (bind _asgs_mejn (cast `/Game/blueprints/GS_Mejn` (`GameplayStatics.GetGameState`)))
  (`BlueprintMapLibrary.Map_Add` (`/Game/blueprints/GS_Mejn.pawnsonboard` _asgs_mejn) self _output_get)
  (bind _asgm_mejn (cast `/Game/blueprints/GM_Mejn` (`GameplayStatics.GetGameMode`)))
  (`/Game/blueprints/GM_Mejn.pawnplacedonboard` _asgm_mejn))

(fn `UserConstructionScript`)