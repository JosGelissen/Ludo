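; Game mode for a four-colour Ludo-style board game (Mejn), running turn order and the rules after each dice throw.
; Starts on a random colour, then gates throwing, boarding and moving through string flags in GS_Mejn's Turnactions map.
; A six boards a pawn while fewer than four are out, otherwise pawns move or the turn passes.
; Events handle hits and house placement, writing per-colour stats back to the game state.
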(event `self.ReceiveBeginPlay`
  (`self.AssignFirstTurn`))

(event `self.ReceiveTick`
  (params (DeltaSeconds :type "Float (single-precision)")))

(event `pawnplacedonboard`
  (`self.disablepawnonboard`)
  (`self.changeturn`))

(event `dicethrown`
  (`self.disablethrowdice`)
  (`self.checkthrow`))

(event `pawnmoved`
  (`self.disablemovepawn`)
  (`self.changeturn`))

(event `pawninhouse`
  (params (pawninhouse :type "/Game/blueprints/yellowpawn Object Reference"))
  (`self.setpawninhouse` pawninhouse))

(event `pawnhit`
  (params (pawn :type "/Game/blueprints/yellowpawn Object Reference"))
  (bind _stats (`self.stats`))
  (`self.K2_DestroyActor` pawn)
  (bind _output_get (set `self.tempint` (- (`BlueprintMapLibrary.Map_Find` _stats "onboard") 1)))
  (`BlueprintMapLibrary.Map_Remove` _stats "onboard")
  (`BlueprintMapLibrary.Map_Add` _stats "onboard" _output_get)
  (`self.updatestats`))

(fn `AssignFirstTurn`
  ;[1 1 1] Set turn to that player
  (bind _asgs_mejn (cast `/Game/blueprints/GS_Mejn` (`GameplayStatics.GetGameState`)))
  (bind _turnactions (`/Game/blueprints/GS_Mejn.turnactions` _asgs_mejn))
  (`BlueprintMapLibrary.Map_Remove` _turnactions "turn")
  (`BlueprintMapLibrary.Map_Add` _turnactions "turn" (`|GetArrayItem` (`self.colorPlayer`) (`KismetMathLibrary.RandomInteger` 4)))
  (`self.enablethrowdice`))

(fn `changeturn`
  (bind _colorplayer (`self.colorPlayer`))
  (bind _asgs_mejn (cast `/Game/blueprints/GS_Mejn` (`GameplayStatics.GetGameState`)))
  (bind _returnvalue (`KismetArrayLibrary.Array_Find` _colorplayer (`BlueprintMapLibrary.Map_Find` (`/Game/blueprints/GS_Mejn.turnactions` _asgs_mejn) "turn")))
  (if (< _returnvalue (- (`KismetArrayLibrary.Array_Length` _colorplayer) 1))
    (set `self.tempstring` (`|GetArrayItem` (`self.colorPlayer`) (+ _returnvalue 1)))
    (else
      (set `self.tempstring` (`|GetArrayItem` (`self.colorPlayer`)))))
  (bind _asgs_mejn_2 (cast `/Game/blueprints/GS_Mejn` (`GameplayStatics.GetGameState`)))
  (bind _turnactions (`/Game/blueprints/GS_Mejn.turnactions` _asgs_mejn_2))
  (`BlueprintMapLibrary.Map_Remove` _turnactions "turn")
  (`BlueprintMapLibrary.Map_Add` _turnactions "turn" (`self.tempstring`))
  (`self.enablethrowdice`))

(fn `checkthrow`
  (bind _stats (`self.stats`))
  (bind _value (`BlueprintMapLibrary.Map_Find` _stats "onboard"))
  (bind _asgs_mejn (cast `/Game/blueprints/GS_Mejn` (`GameplayStatics.GetGameState`)))
  (switch `string` (`BlueprintMapLibrary.Map_Find` (`/Game/blueprints/GS_Mejn.turnactions` _asgs_mejn) "turn")
    (:`yellow`
      (set `self.stats` (`/Game/blueprints/GS_Mejn.yellowstats` _asgs_mejn)))
    (:`green`
      (set `self.stats` (`/Game/blueprints/GS_Mejn.greenstats` _asgs_mejn)))
    (:`blue`
      (set `self.stats` (`/Game/blueprints/GS_Mejn.bluestats` _asgs_mejn)))
    (:`red`
      (set `self.stats` (`/Game/blueprints/GS_Mejn.redstats` _asgs_mejn))))
  (bind _outactors (`GameplayStatics.GetAllActorsOfClass` "/Game/blueprints/BP_Dice.BP_Dice_C"))
  (if (== (`/Game/blueprints/BP_Dice.dicethrow` (`|GetArrayItem` _outactors)) 6)
    ;[1 1 1] If a 6 was thrown: check if player has pawns in house
    (if (< _value 4)
      (`self.enablepawnonboard`)
      (set `self.tempint` _value)
      (`BlueprintMapLibrary.Map_Remove` _stats "onboard")
      (`BlueprintMapLibrary.Map_Add` _stats "onboard" (+ _value 1))
      (`self.updatestats`)
      (else
        (`self.enablemovepawn`)))
    (else
      ;[1 1 1] If no 6 was thrown, check if player has pawn on the board
      (if (> _value 0)
        (`self.enablemovepawn`)
        (else
          (`self.changeturn`)
          (`KismetSystemLibrary.PrintString` "changeturn"))))))

(fn `disablemovepawn`
  (bind _asgs_mejn (cast `/Game/blueprints/GS_Mejn` (`GameplayStatics.GetGameState`)))
  (bind _turnactions (`/Game/blueprints/GS_Mejn.turnactions` _asgs_mejn))
  (`BlueprintMapLibrary.Map_Remove` _turnactions "movepawn")
  (`BlueprintMapLibrary.Map_Add` _turnactions "movepawn" "false"))

(fn `disablepawnonboard`
  (bind _asgs_mejn (cast `/Game/blueprints/GS_Mejn` (`GameplayStatics.GetGameState`)))
  (bind _turnactions (`/Game/blueprints/GS_Mejn.turnactions` _asgs_mejn))
  (`BlueprintMapLibrary.Map_Remove` _turnactions "goonboard")
  (`BlueprintMapLibrary.Map_Add` _turnactions "goonboard" "false"))

(fn `disablethrowdice`
  (bind _asgs_mejn (cast `/Game/blueprints/GS_Mejn` (`GameplayStatics.GetGameState`)))
  (bind _turnactions (`/Game/blueprints/GS_Mejn.turnactions` _asgs_mejn))
  (`BlueprintMapLibrary.Map_Remove` _turnactions "throwdice")
  (`BlueprintMapLibrary.Map_Add` _turnactions "throwdice" "false"))

(fn `enablemovepawn`
  (bind _asgs_mejn (cast `/Game/blueprints/GS_Mejn` (`GameplayStatics.GetGameState`)))
  (bind _turnactions (`/Game/blueprints/GS_Mejn.turnactions` _asgs_mejn))
  (`BlueprintMapLibrary.Map_Remove` _turnactions "movepawn")
  (`BlueprintMapLibrary.Map_Add` _turnactions "movepawn" "true"))

(fn `enablepawnonboard`
  (bind _asgs_mejn (cast `/Game/blueprints/GS_Mejn` (`GameplayStatics.GetGameState`)))
  (bind _turnactions (`/Game/blueprints/GS_Mejn.turnactions` _asgs_mejn))
  (`BlueprintMapLibrary.Map_Remove` _turnactions "goonboard")
  (`BlueprintMapLibrary.Map_Add` _turnactions "goonboard" "true"))

(fn `enablethrowdice`
  (bind _asgs_mejn (cast `/Game/blueprints/GS_Mejn` (`GameplayStatics.GetGameState`)))
  (bind _turnactions (`/Game/blueprints/GS_Mejn.turnactions` _asgs_mejn))
  (`BlueprintMapLibrary.Map_Remove` _turnactions "throwdice")
  (`BlueprintMapLibrary.Map_Add` _turnactions "throwdice" "true"))

(fn `setpawninhouse`
  (params (pawn :type "/Game/blueprints/yellowpawn Object Reference"))
  (bind _stats (`self.stats`))
  (bind _value (`BlueprintMapLibrary.Map_Find` _stats "inhouse"))
  (bind _asgs_mejn (cast `/Game/blueprints/GS_Mejn` (`GameplayStatics.GetGameState`)))
  (bind _outactors (`GameplayStatics.GetAllActorsWithTag` (`KismetStringLibrary.Conv_StringToName` (`BlueprintMapLibrary.Map_Find` (`/Game/blueprints/GS_Mejn.turnactions` _asgs_mejn) "turn"))))
  (`self.K2_SetActorLocation` pawn (`self.K2_GetActorLocation` (`|GetArrayItem` _outactors _value)) false false)
  (bind _output_get (set `self.tempint` (+ _value 1)))
  (`BlueprintMapLibrary.Map_Remove` _stats "inhouse")
  (`BlueprintMapLibrary.Map_Add` _stats "inhouse" _output_get)
  (`self.updatestats`)
  (`BlueprintMapLibrary.Map_Remove` (`/Game/blueprints/GS_Mejn.pawnsonboard` _asgs_mejn) pawn)
  (`self.changeturn`))

(fn `updatestats`
  (bind _stats (`self.stats`))
  (bind _asgs_mejn (cast `/Game/blueprints/GS_Mejn` (`GameplayStatics.GetGameState`)))
  (switch `string` (`BlueprintMapLibrary.Map_Find` (`/Game/blueprints/GS_Mejn.turnactions` _asgs_mejn) "turn")
    (:`yellow`
      (set `/Game/blueprints/GS_Mejn.yellowstats` _stats _asgs_mejn))
    (:`green`
      (set `/Game/blueprints/GS_Mejn.greenstats` _stats _asgs_mejn))
    (:`blue`
      (set `/Game/blueprints/GS_Mejn.bluestats` _stats _asgs_mejn))
    (:`red`
      (set `/Game/blueprints/GS_Mejn.redstats` _stats _asgs_mejn))))

(fn `UserConstructionScript`)