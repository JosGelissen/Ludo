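; Clickable dice actor for the Mejn game that plays a throw animation and rolls a number from 1 to 6.
; Clicking the cube only works while the GS_Mejn game state's Turnactions map has "throwdice" set to "true".
; A vector timeline drives the cube's height, roll and pitch while X and Y stay fixed.
; When it finishes, the random result is stored in Dicethrow and GM_Mejn is notified through Dicethrown.
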(event `self.Cube.OnClicked`
  (params (TouchedComponent :type "PrimitiveComponent Object Reference") (ButtonPressed :type "Key Structure"))
  (bind (_origin_x _origin_y) (`KismetMathLibrary.BreakVector` (`self.origin`)))
  (bind _asgs_mejn (cast `/Game/blueprints/GS_Mejn` (`GameplayStatics.GetGameState`)))
  (if (`KismetStringLibrary.EqualEqual_StrStr` (`BlueprintMapLibrary.Map_Find` (`/Game/blueprints/GS_Mejn.turnactions` _asgs_mejn) "throwdice") "true")
    (set `self.origin` (`SceneComponent.K2_GetComponentLocation` (`self.Cube`)))
    (bind (_direction _newtrack_0) (`Timeline|dicetrow` :!via `PlayFromStart`)
      (:`Update`
        (`SceneComponent.K2_SetWorldLocationAndRotation` (`self.Cube`) (`KismetMathLibrary.MakeVector` _origin_x _origin_y (.z _newtrack_0)) (`KismetMathLibrary.MakeRotator` (.x _newtrack_0) (.y _newtrack_0)) false false))
      (:`Finished`
        (set `self.dicethrow` (`KismetMathLibrary.RandomIntegerInRange` 1 6))
        (bind _asgm_mejn (cast `/Game/blueprints/GM_Mejn` (`GameplayStatics.GetGameMode`)))
        (`/Game/blueprints/GM_Mejn.dicethrown` _asgm_mejn)))))

(fn `UserConstructionScript`)